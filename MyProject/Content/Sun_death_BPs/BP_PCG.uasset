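; BP_PCG is a simple procedural spawner that scatters BP_LogWall actors over a flat grid when play begins.
; Nested loops over GridWidth and GridSize place a wall at each cell, spaced by Scale from the actor's location with a fixed rotation.
; Each scale axis independently rolls 1 with a one-in-four chance, otherwise 0, so most spawned walls are collapsed on at least one axis.
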(event EventBeginPlay
  (bind _returnvalue (Math|Random|RandomIntegerinRange 0 3))
  (bind _scale (Variables|Default|GetScale))
  (bind _returnvalue_2 (> _returnvalue 2))
  (bind _returnvalue_3 (Math|Conversions|ToFloat(Boolean) _returnvalue_2))
  (for _index (range 0 (Variables|Default|GetGridWidth))
    (for _index_2 (range 0 (Variables|Default|GetGridSize))
      (bind _output_get (Variables|Default|SetNext_Position (+ (Math|Vector|MakeVector (* (Math|Conversions|ToFloat(Integer) _index_2) _scale) (* (Math|Conversions|ToFloat(Integer) _index) _scale) 0.0) (Transformation|GetActorLocation))))
      (Game|SpawnActorfromClass "/Game/Sun_death_BPs/BP_LogWall.BP_LogWall_C" (Math|Transform|MakeTransform _output_get "0.000000,90.000000,0.000000" (Math|Vector|MakeVector _returnvalue_3 _returnvalue_3 _returnvalue_3)) "Undefined" "MultiplyWithRoot" 0 0))))

(fn ConstructionScript)